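; Base explosion actor that deals radial damage once, when it spawns.
; On BeginPlay, the server scans all BF4_BasePossess actors and damages those within ExplosionRadius, crediting the instigator's controller.
; Damage is ExplosionDamage scaled by DamageCurve sampled at normalized distance, with no line-of-sight check.
; Debug prints log every scanned actor and each one hit; the Blueprint has no visual or cleanup logic.
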(event `self.ReceiveBeginPlay`
  (bind _explosionradius (`self.ExplosionRadius`))
  (`/Engine/EditorBlueprintResources/ActorMacros.Switch Has Authority`
    (:`Authority`
      (bind _outactors (`GameplayStatics.GetAllActorsOfClass` "/BF4/Vehicles/Possess/BF4_BasePossess.BF4_BasePossess_C"))
      (for _array_element _outactors
        (`KismetSystemLibrary.PrintString` (`KismetSystemLibrary.GetDisplayName` _array_element))
        (bind _returnvalue (`self.GetDistanceTo` _array_element self))
        (if (<= _returnvalue _explosionradius)
          (`KismetSystemLibrary.PrintString` (`KismetSystemLibrary.GetDisplayName` _array_element))
          (`GameplayStatics.ApplyDamage` _array_element (* (`CurveFloat.GetFloatValue` (`self.DamageCurve`) (/ _returnvalue _explosionradius)) (`self.ExplosionDamage`)) (`self.GetInstigatorController`) self (`self.DamageType`)))))))

(fn `UserConstructionScript`)