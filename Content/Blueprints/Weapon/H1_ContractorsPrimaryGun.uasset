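; Contractors primary VR gun Blueprint, extending a parent gun class with custom automatic-fire audio and grip rules.
; For local high-RPM full-auto fire, an attached loop replaces per-shot sounds, fading on fire end or ungrab, with a tail sound after multiple shots.
; The foregrip requires the primary grip to be held, and infinite ammo blocks all interaction.
; Clip installation and firing-direction overrides print debug text; spread is unimplemented.
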(event `self.OnAttachmentInstalled`
  (params (Attachment :type "ZomboyGunAttachment Object Reference"))
  (bind _ascontractors_gun_clip (cast `/Game/Core/VRInteractables/ZomboyGunSystem/Guns/Base/ContractorsGunClip` Attachment))
  (`KismetSystemLibrary.PrintString` (`KismetSystemLibrary.GetDisplayName` _ascontractors_gun_clip)))

(event `self.ReceiveBeginPlay`
  (`parent.ReceiveBeginPlay`))

(event `self.ReceiveDestroyed`
  (`parent.ReceiveDestroyed`))

(event `self.ReceiveTick`
  (params (DeltaSeconds :type "Float (single-precision)"))
  (`parent.ReceiveTick` DeltaSeconds))

(event `self.SpawnFiringSoundEffect`
  (params (Location :type "Vector Structure"))
  (bind _shotloopac (`self.ShotLoopAC`))
  (if (`self.IsLocallyControlled`)
    (`/Engine/EditorBlueprintResources/StandardMacros.IsValid` (`self.LoopSoundCue`)
      (:`Is Valid`
        (if (and (`|EnumEquality` (`self.GetCurrentFiringMode`) "EGunFiringMode_FullAuto") (> (`.FiringRate` (break `ZomboyGunData` (`self.GunData`))) 650))
          (`/Engine/EditorBlueprintResources/StandardMacros.IncrementInt` (`self.ShotsFired`)
            (:`  `
              (`/Engine/EditorBlueprintResources/StandardMacros.DoOnce` false :!label _label
                (:`Completed`
                  (`/Engine/EditorBlueprintResources/StandardMacros.IsValid` (`self.ShotLoopAC`)
                    (:`Is Valid`
                      _)
                    (:`Is Not Valid`
                      (bind _returnvalue (`GameplayStatics.SpawnSoundAttached` (`self.LoopSoundCue`) (`self.GunBodyMesh`) "None" (0.0 0.0 0.0) (struct) "KeepRelativeOffset" true 1.0 1.0 0.0 null null))
                      (set `self.ShotLoopAC` _returnvalue)))
                  (`AudioComponent.Play` _shotloopac 0.0)
                  (`AudioComponent.SetVolumeMultiplier` _shotloopac (`KismetMathLibrary.SelectFloat` (`self.LocalFireCueVolume`) 1.0 (`self.IsLocallyControlled`)))))))
          (else
            (`parent.SpawnFiringSoundEffect` Location :!label _label_2))))
      (:`Is Not Valid`
        (goto _label_2)))
    (else
      (goto _label_2))))

(event `self.EndFullAutoFire`
  (`parent.EndFullAutoFire`)
  (if (`self.IsLocallyControlled`)
    (`|ExecutionSequence`
      (:`then_0`
        (goto _label :!via `Reset`))
      (:`then_1`
        (`/Engine/EditorBlueprintResources/StandardMacros.IsValid` (`self.ShotLoopAC`)
          (:`Is Valid`
            (`AudioComponent.FadeOut` (`self.ShotLoopAC`) 0.3 0.0 "Logarithmic"))))
      (:`then_2`
        (if (> (`self.ShotsFired`) 1)
          (if (`self.IsLocallyControlled`)
            (bind _returnvalue (`GameplayStatics.SpawnSoundAtLocation` "/Game/Sounds/NewWeaponSounds/SFX/LoopEnd/LoopEndSound_Cue.LoopEndSound_Cue" (`SceneComponent.K2_GetComponentLocation` (`self.GunBodyMesh`)) (struct) 1.0 1.0 0.0 null null)))))
      (:`then_3`
        (set `self.ShotsFired` 0)))))

(event `self.OnUngrabbed`
  (params (PrevState :type "InteractibleState Structure (by ref)") (CurrentState :type "InteractibleState Structure (by ref)"))
  (`parent.OnUngrabbed` PrevState CurrentState)
  (`|ExecutionSequence`
    (:`then_0`
      (`/Engine/EditorBlueprintResources/StandardMacros.IsValid` (`self.ShotLoopAC`)
        (:`Is Valid`
          (`AudioComponent.FadeOut` (`self.ShotLoopAC`) 0.3 0.0 "Logarithmic"))))
    (:`then_1`
      (`KismetSystemLibrary.Delay` 0.2)
      (`self.SetActorTickEnabled` true))))

(event `ZomboyAIWeaponInterface.EndFullAutoFiring`
  (`parent.EndFullAutoFiring`)
  (`/Engine/EditorBlueprintResources/StandardMacros.IsValid` (`self.ShotLoopAC`)
    (:`Is Valid`
      (`AudioComponent.FadeOut` (`self.ShotLoopAC`) 0.3 0.0 "Logarithmic"))))

(fn `CanBeginInteraction`
  (params (InteractionComponent :type "ZomboyInteractionComponent Object Reference") (MotionController :type "ZomboyMotionControllerComponent Object Reference"))
  (returns (ReturnValue :type Boolean))
  (bind _returnvalue (`parent.CanBeginInteraction` InteractionComponent MotionController))
  (if (not (`self.bInfiniteAmmo`))
    (if (== InteractionComponent (`self.ForeGripComponent`))
      (return (and _returnvalue (`ZomboyInteractionComponent.IsInteracting` (`self.PrimGripComponent`))))
      (else
        (return _returnvalue)))
    (else
      (return false))))

(fn `GetGunFiringLocationAndDirection`
  (returns (OutLocation :type "Vector Structure") (OutDirection :type "Vector Structure"))
  (bind (_outlocation _outdirection) (`parent.GetGunFiringLocationAndDirection`))
  (`KismetSystemLibrary.PrintString` (`KismetStringLibrary.Concat_StrStr` "Current Spread: " (`KismetStringLibrary.Conv_DoubleToString` 0.0)) true true (struct :`R` 0.538177 :`G` 1.0 :`A` 1.0) 5.0)
  (return _outlocation _outdirection))

(fn `UserConstructionScript`
  (`parent.UserConstructionScript`))