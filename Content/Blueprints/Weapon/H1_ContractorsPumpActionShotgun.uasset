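; VR pump-action shotgun weapon, also exposing attack range, interval and accuracy data for AI.
; Holding the foregrip trigger slides the pump by projecting hand movement onto its clamped axis, with haptics.
; End-of-travel DoOnce gates drive the bolt, ejecting and opening side loading at the back, chambering at the front.
; The server reports gunshot and throttled impact noises and spawns attachments; fire modes fall back from auto to burst to single.
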(event `self.ReceiveBeginPlay`
  (`parent.ReceiveBeginPlay`)
  (`|ExecutionSequence`
    (:`then_0`
      (add `self.OnWeaponFiredEvent` (delegate `OnWeaponFiredEvent_Event_0`))
      (add `self.OnBulletHitEvent` (delegate `OnBulletHitEvent_Event_0`)))
    (:`then_1`
      (`ZomboyInteractionComponent.RegisterHandIKIndicator` (`self.ForeGripComponent`) (`self.RifleForeGripIndicator`) "None" null))))

(event `OnWeaponFiredEvent_Event_0`
  (`/Engine/EditorBlueprintResources/ActorMacros.Switch Has Authority`
    (:`Authority`
      (bind _aspawn (cast `Pawn` (`self.GetOwner`)))
      (`AISense_Hearing.ReportNoiseEvent` (`self.K2_GetActorLocation`) 1.0 _aspawn 100000.0 "GunNoise"))))

(event `OnBulletHitEvent_Event_0` :!signature `self.OnBulletHitEvent`
  (params (HitResult :type "HitResult Structure (by ref)"))
  (`/Engine/EditorBlueprintResources/ActorMacros.Switch Has Authority`
    (:`Authority`
      (`/Engine/EditorBlueprintResources/StandardMacros.DoOnce` false :!label _label
        (:`Completed`
          (`|ExecutionSequence`
            (:`then_0`
              (bind _aspawn (cast `Pawn` (`self.GetOwner`)))
              (`AISense_Hearing.ReportNoiseEvent` (`.Location` (`GameplayStatics.BreakHitResult` HitResult)) 1.0 _aspawn 0.0 "BulletImpact"))
            (:`then_1`
              (`KismetSystemLibrary.Delay` 0.2)
              (goto _label :!via `Reset`))))))))

(event `ServerSpawnAttachments`
  (params (Attachments :type "Array of ZomboyAttachmentInteractable Class Reference") (GunStockCalibrationInfo :type "GunStockCalibrationInfo Structure"))
  (set `self.GunStockCalibrationInfo` GunStockCalibrationInfo)
  (for _array_element Attachments
    (if (`KismetSystemLibrary.IsValidClass` _array_element)
      (bind _returnvalue (`|SpawnActorFromClass` _array_element (`self.GetTransform`) "Undefined" "OverrideRootScale" self null))
      (`self.AuthoritySetAttachment` _returnvalue (`self.GunBodyMesh`) (`ZomboyAttachmentInteractable.GetAttachmentSocketName` _returnvalue) (`KismetMathLibrary.MakeTransform` (0.0 0.0 0.0))))))

(event `self.ParticleCollideEvent`
  (params (EventName :type Name) (EmitterTime :type "Float (single-precision)") (ParticleTime :type Integer) (Location :type "Vector Structure") (Velocity :type "Vector Structure") (Direction :type "Vector Structure") (Normal :type "Vector Structure") (BoneName :type Name) (PhysMat :type "PhysicalMaterial Object Reference"))
  (`GameplayStatics.PlaySoundAtLocation` "/Game/Sounds/Weapon/ShellBounce/shotgun_shell_drop_Cue.shotgun_shell_drop_Cue" Location (struct) 0.7 1.0 0.0 "/Game/ThirdPartyResources/Models/MilitaryWeapSilver/Sound/Attenuation/ProjectileImpact_att.ProjectileImpact_att" null null))

(event `self.OnHandGrabbed`
  (params (MotionController :type "ZomboyMotionControllerComponent Object Reference"))
  (bind _returnvalue (`self.GetCurrentClip`))
  (`|ExecutionSequence`
    (:`then_0`
      (`/Game/Core/ZomboyMacro.IsRunningOnMobile`
        (:`true`
          (if (`self.IsLocallyControlled`)
            (`StaticMeshComponent.SetForcedLodModel` (`self.GunBodyMesh`) 0)
            (`/Engine/EditorBlueprintResources/StandardMacros.IsValid` _returnvalue
              (:`Is Valid`
                (`StaticMeshComponent.SetForcedLodModel` (`ZomboyGunClip.MagazineMesh` _returnvalue) 0)))))))
    (:`then_1`
      (if (`ZomboyMotionControllerComponent.IsLocallyControlled` MotionController)
        (set `SceneComponent.bUseAttachParentBound` false (`self.GunBodyMesh`))
        (else
          (set `SceneComponent.bUseAttachParentBound` true (`self.GunBodyMesh`)))))))

(event `self.ReceiveTick`
  (params (DeltaSeconds :type "Float (single-precision)"))
  (`parent.ReceiveTick` DeltaSeconds))

(event `ZomboyAIWeaponInterface.EndFullAutoFiring`
  (`self.EndFullAutoFire`))

(event `ZomboyAIWeaponInterface.StartFiring`
  (params (FiringMode :type "EGunFiringMode Enum" :default "EGunFiringMode_FullAuto"))
  (switch `EGunFiringMode` FiringMode
    (:`EGunFiringMode_FullAuto`
      (if (`self.SupportFiringMode` "EGunFiringMode_FullAuto")
        (`self.StartFullAutoFire`)
        (else
          (if (`self.SupportFiringMode` "EGunFiringMode_Burst") :!label _label_2
            (`self.StartBurstFire`)
            (else
              (`self.StartSingleFire` :!label _label_3))))))
    (:`EGunFiringMode_Burst`
      (goto _label_2))
    (:`EGunFiringMode_Single`
      (goto _label_3))))

(event `ZomboyAIWeaponInterface.ReloadWeapon`
  (`self.InstantRefillAmmo`))

(event `self.ForeGripComponent.OnHandInteractionBeginEvent`
  (params (Interaction :type "Interaction Structure (by ref)"))
  (set `self.bPumpActionEnabled` false))

(event `self.ForeGripComponent.OnHandInteractionEndEvent`
  (params (Interaction :type "Interaction Structure (by ref)"))
  (set `self.bPumpActionEnabled` false))

(event `self.ForeGripComponent.OnTriggerPressedEvent`
  (params (MotionController :type "ZomboyMotionControllerComponent Object Reference"))
  (`/Engine/EditorBlueprintResources/StandardMacros.IsValid` MotionController
    (:`Is Valid`
      (set `self.bPumpActionEnabled` true)
      (set `self.CachedPumpStartControllerRelativeLocation` (`KismetMathLibrary.InverseTransformLocation` (`self.GetTransform`) (`SceneComponent.K2_GetComponentLocation` MotionController)))
      (set `self.CachedPumpMeshRelativeLocation` (`SceneComponent.RelativeLocation` (`self.PumpStaticMesh`))))))

(event `self.ForeGripComponent.OnTriggerReleasedEvent`
  (params (MotionController :type "ZomboyMotionControllerComponent Object Reference"))
  (set `self.bPumpActionEnabled` false))

(event `self.OnUngrabbed`
  (params (PrevState :type "InteractibleState Structure (by ref)") (CurrentState :type "InteractibleState Structure (by ref)"))
  (`parent.OnUngrabbed` PrevState CurrentState)
  (`KismetSystemLibrary.Delay` 0.2)
  (`self.SetActorTickEnabled` true))

(event `self.ForeGripComponent.OnPreGripUpdateEvent`
  (params (DeltaTime :type "Float (single-precision)") (Interaction :type "Interaction Structure (by ref)"))
  (bind _transform_location (`KismetMathLibrary.BreakTransform` (`ZomboyInteractionLibrary.GetMotionControllerTransformActorSpace` Interaction)))
  (bind _pumpstaticmesh (`self.PumpStaticMesh`))
  (bind _pumpstartrelativelocation_x (`KismetMathLibrary.BreakVector` (`self.PumpStartRelativeLocation`)))
  (bind _pumpendrelativelocation_x (`KismetMathLibrary.BreakVector` (`self.PumpEndRelativeLocation`)))
  (bind _returnvalue (* (`KismetMathLibrary.Abs` (- _pumpstartrelativelocation_x _pumpendrelativelocation_x)) 0.05))
  (bind _returnvalue_2 (`KismetMathLibrary.MakeVector` (`KismetMathLibrary.FClamp` (.x (+ (`KismetMathLibrary.ProjectVectorOnToVector` (- _transform_location (`self.CachedPumpStartControllerRelativeLocation`)) (- (`self.PumpStartRelativeLocation`) (`self.PumpEndRelativeLocation`))) (`self.CachedPumpMeshRelativeLocation`))) _pumpendrelativelocation_x _pumpstartrelativelocation_x) (.y (+ (`KismetMathLibrary.ProjectVectorOnToVector` (- _transform_location (`self.CachedPumpStartControllerRelativeLocation`)) (- (`self.PumpStartRelativeLocation`) (`self.PumpEndRelativeLocation`))) (`self.CachedPumpMeshRelativeLocation`))) (.z (+ (`KismetMathLibrary.ProjectVectorOnToVector` (- _transform_location (`self.CachedPumpStartControllerRelativeLocation`)) (- (`self.PumpStartRelativeLocation`) (`self.PumpEndRelativeLocation`))) (`self.CachedPumpMeshRelativeLocation`)))))
  (bind _x (.x _returnvalue_2))
  (if (and (`self.bPumpActionEnabled`) (`ZomboyInteractionLibrary.IsValid` Interaction))
    (`|ExecutionSequence`
      (:`then_0`
        (set `self.bCanPlayHaptic` (!= (`SceneComponent.RelativeLocation` _pumpstaticmesh) _returnvalue_2 :`ErrorTolerance` 0.07))
        (`SceneComponent.K2_SetRelativeLocation` _pumpstaticmesh _returnvalue_2 false false)
        (`|ExecutionSequence`
          (:`then_0`
            (if (< _x (+ _returnvalue _pumpendrelativelocation_x))
              (`/Engine/EditorBlueprintResources/StandardMacros.DoOnce` false :!label _label_4
                (:`Completed`
                  (`self.OnPumpPumpedBack`)
                  (goto _label_5 :!via `Reset`)))))
          (:`then_1`
            (if (> _x (- _pumpstartrelativelocation_x _returnvalue))
              (`/Engine/EditorBlueprintResources/StandardMacros.DoOnce` false :!label _label_5
                (:`Completed`
                  (`self.OnPumpedForward`)
                  (goto _label_4 :!via `Reset`)))))))
      (:`then_1`
        (if (`self.bCanPlayHaptic`)
          (`ZomboyMotionControllerComponent.PlayHapticFeedback` (`ZomboyInteractionLibrary.GetInteractingMotionController` Interaction) (`self.PumpHapticEffect`)))))))

(event `OnPumpedForward`
  (`PrimitiveComponent.SetCollisionEnabled` (`self.SideBulletInstallCollision`) "NoCollision")
  (`ZomboyGunBoltComponent.BoltTravelToClose` (`self.GunBoltComponent`) 0.0)
  (if (not (`self.HasBulletInChamber`))
    (`self.MoveBulletToChamber`)))

(event `OnPumpPumpedBack`
  (`PrimitiveComponent.SetCollisionEnabled` (`self.SideBulletInstallCollision`) "QueryOnly")
  (`ZomboyGunBoltComponent.BoltTravelToOpen` (`self.GunBoltComponent`) 0.0)
  (`self.EjectChamberBullet`))

(fn `GetAccuracyCurve`
  (returns (ReturnValue :type "CurveFloat Object Reference"))
  (return (`self.AOD_Curve`)))

(fn `GetAnimationOverlay`
  (returns (ReturnValue :type "EZomboyAIOverlay Enum"))
  (return "RIfle"))

(fn `GetAttachmentSocket`
  (returns (ReturnValue :type Name))
  (return "WeapnTransform_R"))

(fn `GetAttackInterval`
  (returns (ReturnValue :type "ZomboyAIWeaponAttackInterval Structure"))
  (return (`self.AIAttackInterval`)))

(fn `GetAttackRange`
  (returns (ReturnValue :type "ZomboyAIWeaponAttackRange Structure"))
  (return (`self.AIAttackRange`)))

(fn `GetGunFiringLocationAndDirection`
  (returns (OutLocation :type "Vector Structure") (OutDirection :type "Vector Structure"))
  (bind (_outlocation _outdirection) (`parent.GetGunFiringLocationAndDirection`))
  (`KismetSystemLibrary.PrintString` (`KismetStringLibrary.Concat_StrStr` "Current Spread: " (`KismetStringLibrary.Conv_DoubleToString` 0.0)) true true (struct :`R` 0.538177 :`G` 1.0 :`A` 1.0) 5.0)
  (return _outlocation _outdirection))

(fn `IsOutOfAmmo`
  (params (bAlmost :type Boolean))
  (returns (ReturnValue :type Boolean))
  (return (`self.GetIsOutOfAmmo` bAlmost)))

(fn `UserConstructionScript`)