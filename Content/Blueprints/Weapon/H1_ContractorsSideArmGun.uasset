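; Contractor's sidearm gun Blueprint, a child weapon that mostly defers to its parent gun class.
; When ungrabbed, it runs the parent handler, then re-enables actor tick after a short delay.
; Its firing location and direction override prints a debug spread readout fixed at zero and returns the parent's values unchanged.
; A random spread rotation is left unconnected, so this class adds no spread.
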(event `self.OnUngrabbed`
  (params (PrevState :type "InteractibleState Structure (by ref)") (CurrentState :type "InteractibleState Structure (by ref)"))
  (`parent.OnUngrabbed` PrevState CurrentState)
  (`KismetSystemLibrary.Delay` 0.2)
  (`self.SetActorTickEnabled` true))

(event `self.ReceiveTick`
  (params (DeltaSeconds :type "Float (single-precision)"))
  (`parent.ReceiveTick` DeltaSeconds))

(fn `GetGunFiringLocationAndDirection`
  (returns (OutLocation :type "Vector Structure") (OutDirection :type "Vector Structure"))
  (bind (_outlocation _outdirection) (`parent.GetGunFiringLocationAndDirection`))
  (`KismetSystemLibrary.PrintString` (`KismetStringLibrary.Concat_StrStr` "Current Spread: " (`KismetStringLibrary.Conv_DoubleToString` 0.0)) true true (struct :`R` 0.538177 :`G` 1.0 :`A` 1.0) 5.0)
  (return _outlocation _outdirection))

(fn `UserConstructionScript`
  (`parent.UserConstructionScript`))