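; H1_SpreadCalcComponent is a weapon component that picks the current spread from a supplied set of spread values, based on the character's movement state.
; CalculateSpread reads the VR character movement component and uses the jumping spread while falling.
; When walking, it checks speed against StillThreshold, then ADS, then VR crouch to choose between moving or still ADS, hip-crouch and hip-stand values.
; Other movement modes leave NewSpread unchanged.
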(event `CalculateSpread`
  (params (CSChar :type "/Game/Core/Player/CS_Character Object Reference") (Spread :type "/MW_Remastered/Blueprints/Weapon/H1_Spread Structure (by ref)"))
  (bind (_ads_not_moving _ads_moving _hip_stand_not_moving _hip_crouch_not_moving _hip_stand_moving _hip_crouch_moving _jumping) (break `/MW_Remastered/Blueprints/Weapon/H1_Spread` Spread))
  (bind _charactermovement (`Character.CharacterMovement` CSChar))
  (bind _asvrcharacter_movement_component (cast `VRCharacterMovementComponent` _charactermovement))
  (switch `EMovementMode` (`CharacterMovementComponent.MovementMode` _charactermovement)
    (:`MOVE_Walking`
      (if (< (`KismetMathLibrary.VSize` (`MovementComponent.Velocity` _charactermovement)) (`self.StillThreshold`))
        (bind _returnvalue (`VRCharacterMovementComponent.IsADS` _asvrcharacter_movement_component))
        (if _returnvalue
          (set `self.newSpread` _ads_not_moving)
          (else
            (bind _returnvalue_2 (`VRCharacterMovementComponent.IsVRCrouching` _asvrcharacter_movement_component))
            (if _returnvalue_2
              (set `self.newSpread` _hip_crouch_not_moving)
              (else
                (set `self.newSpread` _hip_stand_not_moving)))))
        (elif _returnvalue
          (set `self.newSpread` _ads_moving)
          (elif _returnvalue_2
            (set `self.newSpread` _hip_crouch_moving)
            (else
              (set `self.newSpread` _hip_stand_moving))))))
    (:`MOVE_Falling`
      (set `self.newSpread` _jumping))))