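; H1 weapon holster for holding interactables such as guns, with a detection distance reported for motion controllers.
; On authority, a spawned ZomboyGun with a valid default clip class makes the holster manager spawn that clip in the ammo-tagged slot.
; On every machine, putting an interactable in re-enables its actor tick after a short delay.
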(event `self.ReceiveBeginPlay`
  (`parent.ReceiveBeginPlay`)
  (`|ExecutionSequence`
    (:`then_0`
      (`/Engine/EditorBlueprintResources/ActorMacros.Switch Has Authority`
        (:`Authority`
          (add `self.OnInteractableSpawnedDelegate` (delegate `OnInteractableSpawnedDelegate_Event_0`)))))
    (:`then_1`
      (add `self.OnInteractablePutInDelegate` (delegate `OnInteractablePutInDelegate_Event_0`)))))

(event `OnInteractableSpawnedDelegate_Event_0` :!signature `self.OnInteractableSpawnedDelegate`
  (params (InteractableActor :type "ZomboyInteractableActor Object Reference"))
  (bind _aszomboy_gun (cast `ZomboyGun` InteractableActor))
  (bind _returnvalue (`ZomboyGun.GetDefaultClipClass` _aszomboy_gun))
  (if (`KismetSystemLibrary.IsValidClass` _returnvalue)
    (`ZomboyHolsterManagerComponent.ServerSpawnInteractableInHolster` (`self.GetHolsterManager`) (`self.AmmoTag`) _returnvalue)))

(event `OnInteractablePutInDelegate_Event_0` :!signature `self.OnInteractablePutInDelegate`
  (params (InteractableActor :type "ZomboyInteractableActor Object Reference"))
  (`KismetSystemLibrary.Delay` 0.2)
  (`self.SetActorTickEnabled` InteractableActor true))

(fn `GetDetectionDistance`
  (params (MotionController :type "ZomboyMotionControllerComponent Object Reference"))
  (returns (ReturnValue :type "Float (double-precision)"))
  (return (`self.Detection Distance`)))

(fn `UserConstructionScript`
  (`parent.UserConstructionScript`))